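; Player stats component for BP_ThirdPersonCharacter that tracks health, stamina, XP and level.
; BeginPlay waits a tick, caches the owning character and fills its HUD widget; each stat function then updates that HUD directly.
; Decrease functions return true on depletion, increases cap current health and stamina, and reaching max XP levels up, resetting XP and raising the threshold.
; IncreaseMaxStamina sets the stamina bar from the health ratio.
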(event `self.ReceiveBeginPlay`
  (`KismetSystemLibrary.DelayUntilNextTick`)
  (bind _asbp_third_person_character (cast `/Game/ThirdPerson/Blueprints/BP_ThirdPersonCharacter` (`self.GetOwner`)))
  (set `self.As BP Third Person Character` _asbp_third_person_character)
  (`ProgressBar.SetPercent` (`/Game/game_assets/ui/bp_ui_hud.stamina` (`/Game/ThirdPerson/Blueprints/BP_ThirdPersonCharacter.hud_widget` (`self.As BP Third Person Character`))) (/ (`self.current_stamina`) (`self.max_stamina`)))
  (`ProgressBar.SetPercent` (`/Game/game_assets/ui/bp_ui_hud.health` (`/Game/ThirdPerson/Blueprints/BP_ThirdPersonCharacter.hud_widget` (`self.As BP Third Person Character`))) (/ (`self.current_health`) (`self.max_health`)))
  (`ProgressBar.SetPercent` (`/Game/game_assets/ui/bp_ui_hud.xp_bar` (`/Game/ThirdPerson/Blueprints/BP_ThirdPersonCharacter.hud_widget` (`self.As BP Third Person Character`))) (/ (`self.xp`) (`self.max_xp`)))
  (`TextBlock.SetText` (`/Game/game_assets/ui/bp_ui_hud.xp_text` (`/Game/ThirdPerson/Blueprints/BP_ThirdPersonCharacter.hud_widget` (`self.As BP Third Person Character`))) (`|FormatText` "{current_xp}/{max_xp}" (`self.xp`) (`self.max_xp`)))
  (`TextBlock.SetText` (`/Game/game_assets/ui/bp_ui_hud.level_text` (`/Game/ThirdPerson/Blueprints/BP_ThirdPersonCharacter.hud_widget` (`self.As BP Third Person Character`))) (`KismetTextLibrary.Conv_IntToText` (`self.level`))))

(fn `Decrease Health`
  (params (damage :type "Float (double-precision)"))
  (returns (player_dead :type Boolean))
  (bind _hud_widget (`/Game/ThirdPerson/Blueprints/BP_ThirdPersonCharacter.hud_widget` (`self.As BP Third Person Character`)))
  (if (not (<= (`self.current_health`) 0.0))
    (bind _output_get (set `self.current_health` (- (`self.current_health`) damage)))
    (`ProgressBar.SetPercent` (`/Game/game_assets/ui/bp_ui_hud.health` _hud_widget) (/ _output_get (`self.max_health`)))
    (`TextBlock.SetText` (`/Game/game_assets/ui/bp_ui_hud.health_text` _hud_widget) (`KismetTextLibrary.Conv_DoubleToText` (`self.current_health`) "HalfToEven"))
    (if (<= (`self.current_health`) 0.0)
      _
      (else
        (return false))))
  (return true))

(fn `decrease_stamina`
  (params (`stamina-` :type "Float (double-precision)"))
  (returns (not_stamina_left :type Boolean))
  (if (not (<= (`self.current_stamina`) 0.0))
    (set `self.current_stamina` (- (`self.current_stamina`) `stamina-`))
    (`ProgressBar.SetPercent` (`/Game/game_assets/ui/bp_ui_hud.stamina` (`/Game/ThirdPerson/Blueprints/BP_ThirdPersonCharacter.hud_widget` (`self.As BP Third Person Character`))) (/ (`self.current_stamina`) (`self.max_stamina`)))
    (if (<= (`self.current_stamina`) 0.0)
      _
      (else
        (return false))))
  (return true))

(fn `increase_health`
  (params (`health+` :type "Float (double-precision)"))
  (bind _hud_widget (`/Game/ThirdPerson/Blueprints/BP_ThirdPersonCharacter.hud_widget` (`self.As BP Third Person Character`)))
  (set `self.current_health` (+ (`self.current_health`) `health+`))
  (if (>= (`self.current_health`) (`self.max_health`))
    (set `self.current_health` (`self.max_health`)))
  (`ProgressBar.SetPercent` (`/Game/game_assets/ui/bp_ui_hud.health` _hud_widget) (/ (`self.current_health`) (`self.max_health`)))
  (`TextBlock.SetText` (`/Game/game_assets/ui/bp_ui_hud.health_text` _hud_widget) (`KismetTextLibrary.Conv_DoubleToText` (`self.current_health`) "HalfToEven")))

(fn `increase_level`
  (params (`level+` :type Integer))
  (set `self.level` (+ (`self.level`) `level+`))
  (set `self.max_xp` (+ (`self.max_xp`) 150.0))
  (set `self.xp` 0.0)
  (`TextBlock.SetText` (`/Game/game_assets/ui/bp_ui_hud.level_text` (`/Game/ThirdPerson/Blueprints/BP_ThirdPersonCharacter.hud_widget` (`self.As BP Third Person Character`))) (`KismetTextLibrary.Conv_IntToText` (`self.level`))))

(fn `increase_max_health`
  (params (`health+` :type "Float (double-precision)"))
  (bind _hud_widget (`/Game/ThirdPerson/Blueprints/BP_ThirdPersonCharacter.hud_widget` (`self.As BP Third Person Character`)))
  (set `self.max_health` (+ (`self.max_health`) `health+`))
  (`ProgressBar.SetPercent` (`/Game/game_assets/ui/bp_ui_hud.health` _hud_widget) (/ (`self.current_health`) (`self.max_health`)))
  (`TextBlock.SetText` (`/Game/game_assets/ui/bp_ui_hud.health_text` _hud_widget) (`KismetTextLibrary.Conv_DoubleToText` (`self.current_health`) "HalfToEven")))

(fn `increase_max_stamina`
  (params (`stamina+` :type "Float (double-precision)"))
  (set `self.max_stamina` (+ (`self.max_stamina`) `stamina+`))
  (`ProgressBar.SetPercent` (`/Game/game_assets/ui/bp_ui_hud.stamina` (`/Game/ThirdPerson/Blueprints/BP_ThirdPersonCharacter.hud_widget` (`self.As BP Third Person Character`))) (/ (`self.current_health`) (`self.max_health`))))

(fn `increase_stamina`
  (params (`stamina+` :type "Float (double-precision)"))
  (set `self.current_stamina` (+ (`self.current_stamina`) `stamina+`))
  (if (> (`self.current_stamina`) (`self.max_stamina`))
    (set `self.current_stamina` (`self.max_stamina`)))
  (`ProgressBar.SetPercent` (`/Game/game_assets/ui/bp_ui_hud.stamina` (`/Game/ThirdPerson/Blueprints/BP_ThirdPersonCharacter.hud_widget` (`self.As BP Third Person Character`))) (/ (`self.current_stamina`) (`self.max_stamina`))))

(fn `increase_xp`
  (params (`xp+` :type "Float (double-precision)"))
  (set `self.xp` (+ (`self.xp`) `xp+`))
  (if (>= (`self.xp`) (`self.max_xp`))
    (`self.increase_level` 1))
  (`ProgressBar.SetPercent` (`/Game/game_assets/ui/bp_ui_hud.xp_bar` (`/Game/ThirdPerson/Blueprints/BP_ThirdPersonCharacter.hud_widget` (`self.As BP Third Person Character`))) (/ (`self.xp`) (`self.max_xp`)))
  (`TextBlock.SetText` (`/Game/game_assets/ui/bp_ui_hud.xp_text` (`/Game/ThirdPerson/Blueprints/BP_ThirdPersonCharacter.hud_widget` (`self.As BP Third Person Character`))) (`|FormatText` "{current_xp}/{max_xp}" (`self.xp`) (`self.max_xp`))))