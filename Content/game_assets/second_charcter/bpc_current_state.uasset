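; Character component that holds the current weapon state for bp_character, as a second_wepon enum.
; On BeginPlay it waits one tick, then casts its owner to bp_character and caches the reference.
; WeponChange steps the weapon enum back by one with no explicit wrap handling and prints the new value for debugging.
; Tick is empty, and a leftover CurrentWepon print is unconnected.
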(event `self.ReceiveBeginPlay`
  (`KismetSystemLibrary.DelayUntilNextTick`)
  (bind _asbp_character (cast `/Game/game_assets/second_charcter/bp_character` (`self.GetOwner`)))
  (set `self.As Bp Character` _asbp_character))

(event `self.ReceiveTick`
  (params (DeltaSeconds :type "Float (single-precision)")))

(fn `wepon_change`
  (bind _output_get (set `self.wepon` (cast `/Game/game_assets/second_charcter/second_wepon` (- (`self.wepon`) 1))))
  (`KismetSystemLibrary.PrintString` (`|GetEnumeratorNameAsString` _output_get)))