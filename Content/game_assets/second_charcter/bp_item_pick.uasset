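; A pickup weapon item actor whose mesh is set from ItemModel in the construction script.
; Its PickUP event casts the player character to bp_character, stores it and runs the weapon slot function.
; Based on Slot, that function attaches the Item component itself to the character mesh's pistol or rifle socket and stores it in the matching holder variable.
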(event `/Game/game_assets/second_charcter/bp_interact_2.pick_UP`
  (bind _asbp_character (cast `/Game/game_assets/second_charcter/bp_character` (`GameplayStatics.GetPlayerCharacter` 0)))
  (set `self.As Bp Character` _asbp_character)
  (`self.wepon_slot`))

(fn `UserConstructionScript`
  (`StaticMeshComponent.SetStaticMesh` (`self.item`) (`self.item_model`)))