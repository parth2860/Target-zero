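; Rifle pickup actor that equips itself on a bp_character that overlaps its Box.
; The equip event sets the character's weapon enum and writes its string form into the BpcCurrentState component.
; It then attaches only the Rifle component to the rifle_socket on the character's KnifeAttchMesh, keeping relative transforms, and prints a debug message.
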(event `self.rifle.OnComponentBeginOverlap`
  (params (OverlappedComponent :type "PrimitiveComponent Object Reference") (OtherActor :type "Actor Object Reference") (OtherComp :type "PrimitiveComponent Object Reference") (OtherBodyIndex :type Integer) (bFromSweep :type Boolean) (SweepResult :type "HitResult Structure (by ref)")))

(event `equip_rifle`
  (params (Object :type "Object Object Reference"))
  (bind _asbp_character (cast `/Game/game_assets/second_charcter/bp_character` Object))
  (bind _output_get (set `/Game/game_assets/second_charcter/bp_character.wepon` "NewEnumerator2" _asbp_character))
  (bind _bpc_current_state (`/Game/game_assets/second_charcter/bp_character.bpc_current_state` _asbp_character))
  (bind _output_get_2 (set `/Game/game_assets/second_charcter/bpc_current_state.current_wepon` (`|GetEnumeratorNameAsString` _output_get) _bpc_current_state))
  (set `/Game/game_assets/second_charcter/bpc_current_state.s_current_wepon` (`|MakeArray` _output_get_2) _bpc_current_state)
  (`SceneComponent.K2_AttachToComponent` (`self.rifle`) (`/Game/game_assets/second_charcter/bp_character.knife_attch_mesh` _asbp_character) "rifle_socket" "KeepRelative" "KeepRelative" "KeepRelative" true)
  (`KismetSystemLibrary.PrintString` "rifle_quip"))

(event `self.Box.OnComponentBeginOverlap`
  (params (OverlappedComponent :type "PrimitiveComponent Object Reference") (OtherActor :type "Actor Object Reference") (OtherComp :type "PrimitiveComponent Object Reference") (OtherBodyIndex :type Integer) (bFromSweep :type Boolean) (SweepResult :type "HitResult Structure (by ref)"))
  (`self.equip_rifle` OtherActor))

(fn `UserConstructionScript`)