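; Pistol weapon Blueprint that tracks magazine ammo through Fire and Reload events.
; Fire decrements MagazineSize without an empty check and prints the count; it spawns no projectile or trace.
; Reload waits briefly, then resets the magazine to a hard-coded capacity and prints a debug message.
; A fire animation call on WeponModel is left unconnected, so it never plays.
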(event `/Game/game_assets/interfaces/bpi_fire.fire`
  (bind _output_get (set `self.magazine_size` (- (`self.magazine_size`) 1)))
  (`KismetSystemLibrary.PrintString` (`KismetStringLibrary.Conv_IntToString` _output_get)))

(event `/Game/game_assets/interfaces/bpi_reload.reload`
  (`KismetSystemLibrary.Delay` 1.0)
  (set `self.magazine_size` 10)
  (`KismetSystemLibrary.PrintString` "reload_pistol"))

(fn `UserConstructionScript`
  (`parent.UserConstructionScript`))