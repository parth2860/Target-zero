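; Zombie enemy that chases the player on sight and damages them on contact.
; PawnSensing sets a seeing flag, which is never cleared here, starts an AI MoveTo toward player character 0 and sets walk speed.
; Capsule hits on the third-person character subtract a fixed, clamped amount from CurrentHealth in its Bpc_playerstate component, with no cooldown.
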(event `self.PawnSensing.OnSeePawn`
  (params (Pawn :type "Pawn Object Reference"))
  ;[1 1 1] enemy sense
  (set `self.is_seeing` true)
  (`self.enemy follow`)
  (set `CharacterMovementComponent.MaxWalkSpeed` 100.0 (`self.CharacterMovement`)))

(event `self.PawnSensing.OnHearNoise`
  (params (Instigator :type "Pawn Object Reference") (Location :type "Vector Structure (by ref)") (Volume :type "Float (single-precision)"))
  ;[1 1 1] enemy sense
)

(event `enemy follow`
  ;[1 1 1] enemy follow
  (if (`self.is_seeing`)
    (`|AIMoveTo` self (0.0 0.0 0.0) (`GameplayStatics.GetPlayerCharacter` 0))))

(event `self.CapsuleComponent.OnComponentHit`
  (params (HitComponent :type "PrimitiveComponent Object Reference") (OtherActor :type "Actor Object Reference") (OtherComp :type "PrimitiveComponent Object Reference") (NormalImpulse :type "Vector Structure") (Hit :type "HitResult Structure (by ref)"))
  (bind _returnvalue (`self.GetComponentByClass` (`self.BP Third Person Character`) "/Game/game_assets/player_state/bpc_playerstate.bpc_playerstate_C"))
  ;[1 1 1] enemy interaction
  (bind _asbp_third_person_character (cast `/Game/ThirdPerson/Blueprints/BP_ThirdPersonCharacter` OtherActor))
  (set `self.BP Third Person Character` _asbp_third_person_character)
  (set `/Game/game_assets/player_state/bpc_playerstate.current_health` (`KismetMathLibrary.FClamp` (- (`/Game/game_assets/player_state/bpc_playerstate.current_health` _returnvalue) 20.0) 0.0 100.0) _returnvalue))

(event `self.CapsuleComponent.OnComponentBeginOverlap`
  (params (OverlappedComponent :type "PrimitiveComponent Object Reference") (OtherActor :type "Actor Object Reference") (OtherComp :type "PrimitiveComponent Object Reference") (OtherBodyIndex :type Integer) (bFromSweep :type Boolean) (SweepResult :type "HitResult Structure (by ref)"))
  ;[1 1 1] enemy interaction
)

(fn `UserConstructionScript`)